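; BP_Spawner is a placeable map actor that spawns a turtle on demand and keeps only one of its turtles alive at a time.
; Spawn destroys the current turtle if valid, then spawns TurtleClass at the Capsule's location and stores it.
; It then calls InitControlling on the new turtle, passing a behavior tree and TargetPosition converted from Cylinder-relative to world space.
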(event `self.ReceiveBeginPlay`)

(fn `Spawn`
  (bind _currentturtelobject (`self.CurrentTurtelObject`))
  (`|ExecutionSequence`
    (:`then_0`
      ;[1 0.5546 0.3933] Destroy previous "turtle" if it is on scene :(
      (if (`KismetSystemLibrary.IsValid` _currentturtelobject)
        (`self.K2_DestroyActor` _currentturtelobject)))
    (:`then_1`
      ;[0.5925 1 0.6093] Spawn new "turtle"
      (bind _returnvalue (`|SpawnActorFromClass` (`self.TurtleClass`) (`KismetMathLibrary.Conv_VectorToTransform` (`SceneComponent.K2_GetComponentLocation` (`self.Capsule`))) "Undefined" "OverrideRootScale" null null))
      (set `self.CurrentTurtelObject` _returnvalue))
    (:`then_2`
      ;[0.4125 0.4818 1] Init "turtle"
      (`AICharacter.InitControlling` (`self.CurrentTurtelObject`) (`KismetMathLibrary.TransformLocation` (`SceneComponent.K2_GetComponentToWorld` (`self.Cylinder`)) (`self.TargetPosition`)) (`self.BehaverTree`)))))

(fn `UserConstructionScript`)